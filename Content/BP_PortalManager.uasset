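; Portal manager actor that drives the capture component of a referenced portal from the player's view.
; Every Tick, PortalUpdate moves Portal1's CapturePortal to the player camera's world location and rotation.
; The location offset subtracts Portal1's OuterMesh position from itself, so it is always zero.
; A 180-degree yaw-flip rotation calculation exists but is unconnected.
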(event EventBeginPlay)

(event Collision|EventActorBeginOverlap
  (params (OtherActor :type Actor%20Object%20Reference)))

(event EventTick
  (params (DeltaSeconds :type Float%20%28single-precision%29))
  (CallFunction|PortalUpdate))

(fn ConstructionScript)

(fn PortalUpdate
  (bind _returnvalue (Game|GetPlayerCameraManager 0))
  (bind _portal1 (Variables|Default|GetPortal1))
  (bind _transformcomponent (Variables|/Script/Engine.PlayerCameraManager|GetTransformComponent _returnvalue))
  (bind _outermesh (Variables|/Script/PortalSystem.Portal|GetOuterMesh _portal1))
  (bind _returnvalue_2 (Transformation|GetWorldLocation _outermesh))
  (Transformation|SetWorldLocationAndRotation (Variables|/Script/PortalSystem.Portal|GetCapturePortal (Variables|Default|GetPortal1)) (+ (- _returnvalue_2 _returnvalue_2) (Transformation|GetWorldLocation _transformcomponent)) (Transformation|GetWorldRotation _transformcomponent) false false))